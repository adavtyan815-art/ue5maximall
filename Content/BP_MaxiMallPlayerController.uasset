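; BP_MaxiMallPlayerController is a player controller that shows the mouse cursor when play begins.
; An unconnected chain, which never runs, checks for a valid CurrentBooth and treats two clicks within a short real-time window as a double click that calls HandleDoubleClickInteraction.
; The construction script is empty.
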(event `Key|LeftMouseButton`
  (params (Key :type "Key Structure")))

(event `self.ReceiveBeginPlay`
  (set `self.bShowMouseCursor` true))

(fn `UserConstructionScript`)